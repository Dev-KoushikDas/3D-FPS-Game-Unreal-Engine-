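; Base weapon Blueprint that tracks magazine and reserve ammo.
; WeaponFire removes one round without checking the count; HasAmmoInMag and HasExtraAmmo report whether the magazine has rounds or is full and whether reserve remains.
; WeaponReload sets the magazine to the lesser of its capacity and the reserve, then deducts that amount from the reserve, so rounds left in the magazine are discarded.
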(fn `Has ExtraAmmo`
  (returns (HasExtraAmmo :type Boolean))
  (return (> (`self.CurrentTotalAmmo`) 0)))

(fn `HasAmmoInMag`
  (returns (`HasAmmo?` :type Boolean) (`MagFull?` :type Boolean))
  (return (> (`self.CurrentAmmo`) 0) (== (`self.CurrentAmmo`) (`self.MaxMegAmmo`))))

(fn `UserConstructionScript`)

(fn `WeaponFire`
  (set `self.CurrentAmmo` (- (`self.CurrentAmmo`) 1)))

(fn `WeaponReload`
  (bind _returnvalue (`KismetMathLibrary.Min` (`self.MaxMegAmmo`) (`self.CurrentTotalAmmo`)))
  (set `self.CurrentAmmo` _returnvalue)
  (set `self.CurrentTotalAmmo` (- (`self.CurrentTotalAmmo`) _returnvalue)))